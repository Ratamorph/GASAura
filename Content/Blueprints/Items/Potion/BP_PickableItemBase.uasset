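; Base pickable item for potions that grants Gameplay Ability System effects to an actor that overlaps it.
; On overlap, it passes the other actor to ApplyEffectToTarget twice, once with an instant effect class and once with a duration effect class, then destroys itself.
; A manual effect-spec application through the target's ability system component remains in the graph but is disconnected.
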(event EventBeginPlay)

(event Collision|EventActorBeginOverlap
  (params (OtherActor :type Actor%20Object%20Reference))
  (Class|AuraEffectActor|ApplyEffecttoTarget OtherActor (Variables|Default|GetInstantEffectToApply))
  (Class|AuraEffectActor|ApplyEffecttoTarget OtherActor (Variables|Default|GetDurationEffectToApply))
  (Actor|DestroyActor))

(event EventTick
  (params (DeltaSeconds :type Float%20%28single-precision%29)))

(fn ConstructionScript)