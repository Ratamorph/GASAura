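; BP_AreaEffect is a crystal item Blueprint that acts as an area effect, reacting to actors entering and leaving its overlap.
; Begin and end overlap events pass the other actor to OnOverlap and OnEndOverlap, whose logic is not defined in this graph.
; Disconnected nodes hold an unused Gameplay Ability System version that applies an infinite effect to the actor and removes it through a stored handle.
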(event EventBeginPlay)

(event Collision|EventActorBeginOverlap
  (params (OtherActor :type Actor%20Object%20Reference))
  (Class|AuraEffectActor|OnOverlap OtherActor))

(event Collision|EventActorEndOverlap
  (params (OtherActor :type Actor%20Object%20Reference))
  (Class|AuraEffectActor|OnEndOverlap OtherActor))

(fn ConstructionScript)