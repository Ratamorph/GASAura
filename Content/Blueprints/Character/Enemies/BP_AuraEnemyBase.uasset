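; Base Blueprint for Aura enemies, handling the lifebar, death-style dissolve visual and hit-react montage lookup.
; On BeginPlay it sets itself as the widget controller of its lifebar widget and binds to Health and MaxHealth changes.
; Health changes push a safe-divided health ratio to the lifebar, while MaxHealth changes only cache the value.
; StartDissolveEffect plays a timeline driving the dynamic material's Dissolve parameter, and GetHitReact returns the montage.
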(event Custom|HealthChanged
  (params (NewValue :type Float%20%28single-precision%29))
  (bind _output_get (Variables|Default|SetHealth NewValue))
  (Default|UpdateLifeBar (Variables|Default|GetEnemyLifebarWidget) (Math|Float|SafeDivide _output_get (Variables|Default|GetMaxHealth))))

(event Custom|MaxhealthChanged
  (params (NewValue :type Float%20%28single-precision%29))
  (Variables|Default|SetMaxHealth NewValue))

(event EventBeginPlay
  (bind _aswbp_aura_enemy_lifebar (Utilities|Casting|CastToWBP_AuraEnemyLifebar (UserInterface|GetWidget (Variables|Default|GetWidget))))
  (Variables|Default|SetEnemyLifebarWidget _aswbp_aura_enemy_lifebar)
  (Class|AuraUserWidget|SetWidgetController _aswbp_aura_enemy_lifebar self)
  (EventDispatchers|BindEventtoOnHealthChanged (delegate Custom|HealthChanged))
  (EventDispatchers|BindEventtoOnMaxHealthChanged (delegate Custom|MaxhealthChanged)))

(event EventStartDissolveEffect
  (params (DynamicDissolveMaterial :type Material%20Instance%20Dynamic%20Object%20Reference))
  (bind _dissolveamount (Timeline|DissolveEffect Play)
    (:Update
      (Rendering|Material|SetScalarParameterValue DynamicDissolveMaterial "Dissolve" _dissolveamount :!class /Script/Engine.MaterialInstanceDynamic))))

(fn ConstructionScript)

(fn GetHitReact
  (return (Variables|Default|GetHitReactMontage)))